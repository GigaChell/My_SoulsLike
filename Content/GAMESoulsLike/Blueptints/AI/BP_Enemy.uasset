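; Souls-like enemy character with montage-driven sword and big attacks, a health bar widget and ragdoll death.
; BeginSwordTrace starts a looping timer that sphere-traces between two sword points for pawns until EndSwordTrace, with a DoOnce and short delay throttling hits.
; PointDamageTrace is a separate one-shot sphere check dealing fixed damage.
; Damage taken reduces a BPCStats value, and Die disables movement, enables mesh physics and stops sword hits.
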(event Custom|DAmage%20Trace
  ;[0.15 0.15 0.15 0.5] Sword traces
  (if (not (Variables|Default|GetIsDead?))
    (bind (_outhit _returnvalue) (Collision|SphereTraceForObjects (Transformation|GetWorldLocation (Variables|Default|GetStart%20Position)) (Transformation|GetWorldLocation (Variables|Default|GetEnd%20Position)) (Variables|Default|GetswordAttackRadius) (Utilities|Array|MakeArray "ObjectTypeQuery3") false 0 "ForOneFrame"))
    (if _returnvalue
      (Utilities|FlowControl|DoOnce false :!label _label
        (:Completed
          (Game|Damage|ApplyDamage (.HitActor (Collision|BreakHitResult _outhit)) (Variables|Default|GetSwordDamage) 0 0)
          (Utilities|FlowControl|Delay 0.2)
          (goto _label Reset))))))

(event EventBeginPlay
  (bind _aswb_enemy_health_bar (Utilities|Casting|CastToWB_EnemyHealthBar (UserInterface|GetWidget (Variables|Default|GetWidget))))
  (Default|SetHealthProgressBar (Variables|Default|GetBPC_Stats) (Variables|/Game/GAMESoulsLike/UI/WB_EnemyHealthBar.WB_EnemyHealthBar_C|GetHealthBar _aswb_enemy_health_bar)))

(event EventPointDamageTrace
  (bind _pointtracepos (Variables|Default|GetPointTracePos))
  (bind _returnvalue (Transformation|GetWorldLocation _pointtracepos))
  (bind (_outhit _returnvalue_2) (Collision|SphereTraceForObjects _returnvalue _returnvalue (Variables|Default|GetPointAttackRadius) (Utilities|Array|MakeArray "ObjectTypeQuery3") false 0 "ForDuration" true "(R=1.000000,G=0.000000,B=0.000000,A=1.000000)" "(R=0.000000,G=1.000000,B=0.000000,A=1.000000)" 1.0))
  (if _returnvalue_2
    (Game|Damage|ApplyDamage (.HitActor (Collision|BreakHitResult _outhit)) 1e+01 0 0)))

(event EventEndSwordTrace
  ;[0.15 0.15 0.15 0.5] Sword traces
  (if (Utilities|Time|IsValidTimerHandle (stale EventBeginSwordTrace _returnvalue))
    (Utilities|Time|ClearandInvalidateTimerbyHandle (stale EventBeginSwordTrace _returnvalue))))

(event EventBeginSwordTrace
  ;[0.15 0.15 0.15 0.5] Sword traces
  (bind _returnvalue (Utilities|Time|SetTimerbyEvent (delegate Custom|DAmage%20Trace) 0.01 true)))

(event Game|Damage|EventAnyDamage
  (params (Damage :type Float%20%28single-precision%29) (DamageType :type Damage%20Type%20Object%20Reference) (InstigatedBy :type Controller%20Object%20Reference) (DamageCauser :type Actor%20Object%20Reference))
  (Default|IncreaseValue (Variables|Default|GetBPC_Stats) "NewEnumerator0" (* Damage -1.0)))

(event EventDie
  (Pawn|Components|CharacterMovement|DisableMovement (Variables|Character|GetCharacterMovement))
  (Physics|SetSimulatePhysics (Variables|Character|GetMesh) true)
  (Variables|Default|SetIsDead? true))

(fn ConstructionScript)

(fn BigAttack
  (bind _returnvalue (Animation|PlayAnimMontage (Variables|Default|GetBig%20Anim%20Montage) 1.0 "None"))
  (return _returnvalue))

(fn SwordAttack
  (bind _returnvalue (Animation|PlayAnimMontage (Variables|Default|GetSword%20Anim%20Montage) 1.0 "None"))
  (return _returnvalue))