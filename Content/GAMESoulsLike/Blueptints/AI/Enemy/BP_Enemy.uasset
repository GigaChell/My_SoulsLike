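; BP_Enemy is a Souls-like enemy character with component-driven stats and melee combat.
; BPCCombat runs sword damage traces between begin and end events, while incoming damage lowers a BPCStats value and plays a hit-react montage that halts walking until it ends.
; On BeginPlay it adds a WB_HUD to the viewport and hands its player health bar to BPCStats.
; Die disables movement and ragdolls the mesh; a debug key applies self-damage.
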(event EventBeginPlay
  ;[0.15 0.15 0.15 0.5] Player HUD WIdJET
  (bind _returnvalue (UserInterface|CreateWidget "/Game/GAMESoulsLike/UI/WB_HUD.WB_HUD_C"))
  (bind _output_get (Variables|Default|SetHUDWidjet _returnvalue))
  ;[0.15 0.15 0.15 0.5] Set Health Bar
  (UserInterface|Viewport|AddtoViewport _output_get 0)
  (Default|SetHealthProgressBar (Variables|Default|GetBPC_Stats) (Variables|/Game/GAMESoulsLike/UI/WB_PlayerHealth.WB_PlayerHealth_C|GetHealthBar (Variables|/Game/GAMESoulsLike/UI/WB_HUD.WB_HUD_C|GetWB_PlayerHealth (Variables|Default|GetHUDWidjet)))))

(event Collision|EventActorBeginOverlap
  (params (OtherActor :type Actor%20Object%20Reference)))

(event EventTick
  (params (DeltaSeconds :type Float%20%28single-precision%29)))

(event EventEndSwordTrace
  ;[0.15 0.15 0.15 0.5] Sword Traces
  (Default|EndDamageTrace (Variables|Default|GetBPC_Combat)))

(event EventBeginSwordTrace
  ;[0.15 0.15 0.15 0.5] Sword Traces
  (Default|BeginDamageTrace (Variables|Default|GetBPC_Combat)))

(event Game|Damage|EventAnyDamage
  (params (Damage :type Float%20%28single-precision%29) (DamageType :type Damage%20Type%20Object%20Reference) (InstigatedBy :type Controller%20Object%20Reference) (DamageCauser :type Actor%20Object%20Reference))
  (bind _charactermovement (Variables|Character|GetCharacterMovement))
  (Default|IncreaseValue (Variables|Default|GetBPC_Stats) "NewEnumerator0" (* Damage -1.0))
  (Animation|Montage|PlayMontage (Variables|Character|GetMesh) "/Game/GAMESoulsLike/Animations/Combat/HitReact_Montage.HitReact_Montage"
    (:then
      (Variables|/Script/Engine.CharacterMovementComponent|SetMaxWalkSpeed _charactermovement 0.0))
    (:OnCompleted
      (Variables|/Script/Engine.CharacterMovementComponent|SetMaxWalkSpeed _charactermovement 4.8e+02 :!label _label))
    (:OnInterrupted
      (goto _label))))

(event EventDie
  ;[0.15 0.15 0.15 0.5] Отключвается движение и устанавлявается физика
  (Pawn|Components|CharacterMovement|DisableMovement (Variables|Character|GetCharacterMovement))
  (Physics|SetSimulatePhysics (Variables|Character|GetMesh) true))

(event Input|KeyboardEvents|DebugKeyT
  (params (Key :type Key%20Structure) (ActionValue :type Input%20Action%20Value%20Structure))
  (:Pressed
    (Game|Damage|ApplyDamage self 1e+01 0 0)))

(fn ConstructionScript)