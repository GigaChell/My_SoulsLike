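; Souls-like enemy character with sword combo and big attack montages, a health bar widget, and ragdoll on death.
; While the trace window is open, a looping timer sphere-traces the blade for pawns and applies SwordDamage, gated by a DoOnce with short cooldown.
; Damage taken reduces a BPCStats value; the component drives the health bar.
; BeginPlay sets IsDead true, which blocks damage traces unless cleared elsewhere.
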(event Custom|DAmage%20Trace
  ;[0.15 0.15 0.15 0.5] Sword traces
  (if (not (Variables|Default|GetIsDead?))
    (bind _outhit (Collision|SphereTraceForObjects (Transformation|GetWorldLocation (Variables|Default|GetStart%20Position)) (Transformation|GetWorldLocation (Variables|Default|GetEnd%20Position)) 15.0 (Utilities|Array|MakeArray "ObjectTypeQuery3") false 0 "ForOneFrame"))
    (if true
      (Utilities|FlowControl|DoOnce false :!label _label
        (:Completed
          (Game|Damage|ApplyDamage (.HitActor (Collision|BreakHitResult _outhit)) (Variables|Default|GetSwordDamage) 0 0)
          (Utilities|FlowControl|Delay 0.2)
          (goto _label Reset))))))

(event EventBeginPlay
  (bind _aswb_enemy_health_bar (Utilities|Casting|CastToWB_EnemyHealthBar (UserInterface|GetWidget (Variables|Default|GetWidget))))
  (Default|SetHealthProgressBar (Variables|Default|GetBPC_Stats) (Variables|/Game/GAMESoulsLike/UI/WB_EnemyHealthBar.WB_EnemyHealthBar_C|GetHealthBar _aswb_enemy_health_bar))
  (Variables|Default|SetIsDead? true))

(event EventEndSwordTrace
  ;[0.15 0.15 0.15 0.5] Sword traces
  (if (Utilities|Time|IsValidTimerHandle (stale EventBeginSwordTrace _returnvalue))
    (Utilities|Time|ClearandInvalidateTimerbyHandle (stale EventBeginSwordTrace _returnvalue))))

(event EventBeginSwordTrace
  ;[0.15 0.15 0.15 0.5] Sword traces
  (bind _returnvalue (Utilities|Time|SetTimerbyEvent (delegate Custom|DAmage%20Trace) 0.01 true)))

(event Game|Damage|EventAnyDamage
  (params (Damage :type Float%20%28single-precision%29) (DamageType :type Damage%20Type%20Object%20Reference) (InstigatedBy :type Controller%20Object%20Reference) (DamageCauser :type Actor%20Object%20Reference))
  (Default|IncreaseValue (Variables|Default|GetBPC_Stats) "NewEnumerator0" (* Damage -1.0)))

(event EventDie
  (Pawn|Components|CharacterMovement|DisableMovement (Variables|Character|GetCharacterMovement))
  (Physics|SetSimulatePhysics (Variables|Character|GetMesh) true))

(fn ConstructionScript)

(fn BigAttack
  (Animation|PlayAnimMontage "/Game/GAMESoulsLike/Animations/Combat/BigAttack_Montage.BigAttack_Montage" 1.0 "None")
  (return 0.0))

(fn SwordAttack
  (bind _returnvalue (Animation|PlayAnimMontage "/Game/GAMESoulsLike/Animations/Combat/SwordAttackCombo_Montage.SwordAttackCombo_Montage" 1.0 "None"))
  (return _returnvalue))